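; BP_Tooth is a tooth actor that scales in when play begins and can be repainted in a random color.
; The construction script picks its static mesh from the ToothStaticMesh array using ToothIndex.
; BeginPlay creates a dynamic instance of MI_Teeth and runs a timeline whose Alpha drives the mesh's uniform relative scale.
; PaintRandomColor sets a random RGB BaseColor on that material instance.
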(event Custom|PaintRandomColor
  (Rendering|Material|SetVectorParameterValue (Variables|Default|GetDynMaterial) "BaseColor" (Math|Color|MakeColor (Math|Random|RandomFloatinRange 0.0 1.0) (Math|Random|RandomFloatinRange 0.0 1.0) (Math|Random|RandomFloatinRange 0.0 1.0)) :!class /Script/Engine.MaterialInstanceDynamic))

(event EventBeginPlay
  (bind _returnvalue (Rendering|Material|CreateDynamicMaterialInstance (Variables|Default|GetStaticMesh) 0 "/Game/HF/Materials/Master/MI_Teeth.MI_Teeth" "None" :!class /Script/Engine.PrimitiveComponent))
  (Variables|Default|SetDynMaterial _returnvalue)
  (bind _alpha (Timeline|Timeline PlayFromStart)
    (:Update
      (Transformation|SetRelativeScale3D (Variables|Default|GetStaticMesh) (Math|Conversions|ToVector(Float) _alpha)))))

(fn ConstructionScript
  (Components|StaticMesh|SetStaticMesh (Variables|Default|GetStaticMesh) (Utilities|Array|Get(acopy) (Variables|Default|GetToothStaticMesh) (Variables|Default|GetToothIndex))))