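; Player controller for the dental game BearGrillz, viewing through a fixed BP_Camera and driving the BP_Dentist character.
; Left click traces from the cursor, moves the dentist's hand to the hit and, after a short delay, calls Interact on the current tool.
; Number keys switch tools, triggering a dentist reaction, while holding right click shows the tool menu.
; Escape or P pauses into the main menu until all HUD widgets close.
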(event Custom|Set%20Tool
  (params (ToolID :type Integer))
  (bind _output (CallFunction|GetCurrentTool))
  ;[0.5 0.2956 0 0.5] SetTool
  (Variables|Default|SetCurrentTool ToolID)
  (Default|StartInteract _output)
  (Default|CallOnToolChanged _output)
  (Default|PlayRandomReaction (Variables|Default|GetDentistCharacter)))

(event Custom|OnCloseAllWidgets_Event
  (bind _ashud_bear_grillz (Utilities|Casting|CastToHUD_BearGrillz (HUD|GetHUD)))
  (EventDispatchers|UnbindEventfromOnCloseAllWidgets _ashud_bear_grillz (delegate Custom|OnCloseAllWidgets_Event))
  (Game|SetGamePaused false)
  (Utilities|Time|SetGlobalTimeDilation 1.0)
  (Utilities|FlowControl|DelayUntilNextTick)
  (Input|SetInputModeGameOnly self true)
  (Class|GameplayStatics|SetViewportMouseCaptureMode "CapturePermanently_IncludingInitialMouseDown"))

(event EventBeginPlay
  ;[0 0.445 0.5 0.5] BeginPlay
  (Utilities|FlowControl|Sequence
    (:then_0
      (bind _returnvalue (Actor|GetActorOfClass "/Game/HF/Blueprints/Core/BP_Camera.BP_Camera_C"))
      (bind _output_get (Variables|Default|SetMainCamera _returnvalue))
      (Game|Player|SetViewTargetwithBlend _output_get 0.0 "VTBlend_Linear" 0.0 false)
      (Variables|Default|SetbShowMouseCursor true)
      (bind _returnvalue_2 (Actor|GetActorOfClass "/Game/HF/Characters/Dentist/BP_Dentist.BP_Dentist_C"))
      (Variables|Default|SetDentistCharacter _returnvalue_2))
    (:then_1
      (Variables|Default|SetTools (Utilities|Array|MakeArray (Variables|Default|GetTOOL_Grillz) (Variables|Default|GetTOOL_Extractor) (Variables|Default|GetTOOL_Escurecedor) (Variables|Default|GetTOOL_Brackets) (Variables|Default|GetTOOL_Clareador))))))

(event Input|MouseEvents|LeftMouseButton
  (params (Key :type Key%20Structure :default "None"))
  (bind (_locationx _locationy) (Game|Player|GetMousePosition))
  (bind _self self)
  (bind _returnvalue (Math|Vector2D|MakeVector2D _locationx _locationy))
  (bind (_worldposition _worlddirection) (Class|GameplayStatics|DeprojectScreentoWorld _self _returnvalue))
  ;[0.5 0 0 0.5] Interaction
  (:Pressed
    (bind _outhit (Collision|LineTraceByChannel _worldposition (+ (Transformation|GetActorLocation (Variables|Default|GetMainCamera)) (* _worlddirection 4e+03)) "TraceTypeQuery1" false (Utilities|Array|MakeArray self) "None" true "(R=1.000000,G=0.000000,B=0.000000,A=1.000000)" "(R=0.000000,G=1.000000,B=0.000000,A=1.000000)" 15.0))
    (Utilities|FlowControl|Sequence
      (:then_0
        (bind _returnvalue_2 (Actor|GetActorOfClass "/Game/HF/Characters/Dentist/BP_Dentist.BP_Dentist_C"))
        (Default|MoveHandtoLocation _returnvalue_2 (.Location (Collision|BreakHitResult _outhit))))
      (:then_1
        (Utilities|FlowControl|Delay 0.4)
        (if (.bBlockingHit (Collision|BreakHitResult _outhit))
          (Default|Interact (Utilities|Array|Get(acopy) (Variables|Default|GetTools) (Variables|Default|GetCurrentTool)) _outhit))))))

(event Input|KeyboardEvents|1
  (params (Key :type Key%20Structure :default "None"))
  (:Pressed
    (CallFunction|SetTool)))

(event Input|KeyboardEvents|P
  (params (Key :type Key%20Structure :default "None"))
  (:Pressed
    (bind _ashud_bear_grillz (Utilities|Casting|CastToHUD_BearGrillz (HUD|GetHUD)))
    (EventDispatchers|BindEventtoOnCloseAllWidgets _ashud_bear_grillz (EventDispatchers|CreateEvent :!event Custom|OnCloseAllWidgets_Event))
    (Game|SetGamePaused true)
    (Utilities|Time|SetGlobalTimeDilation 0.0)
    (Default|OpenWidget _ashud_bear_grillz "/Game/HF/Widgets/WBP_MainMenu.WBP_MainMenu_C")))

(event Input|KeyboardEvents|2
  (params (Key :type Key%20Structure :default "None"))
  (:Pressed
    (CallFunction|SetTool 1)))

(event Input|KeyboardEvents|3
  (params (Key :type Key%20Structure :default "None"))
  (:Pressed
    (CallFunction|SetTool 2)))

(event Input|KeyboardEvents|Escape
  (params (Key :type Key%20Structure :default "None"))
  (:Pressed
    (bind _ashud_bear_grillz (Utilities|Casting|CastToHUD_BearGrillz (HUD|GetHUD)))
    (EventDispatchers|BindEventtoOnCloseAllWidgets _ashud_bear_grillz (EventDispatchers|CreateEvent :!event Custom|OnCloseAllWidgets_Event))
    (Game|SetGamePaused true)
    (Utilities|Time|SetGlobalTimeDilation 0.0)
    (Default|OpenWidget _ashud_bear_grillz "/Game/HF/Widgets/WBP_MainMenu.WBP_MainMenu_C")))

(event Input|KeyboardEvents|4
  (params (Key :type Key%20Structure :default "None"))
  (:Pressed
    (CallFunction|SetTool 3)))

(event Input|KeyboardEvents|5
  (params (Key :type Key%20Structure :default "None"))
  (:Pressed
    (CallFunction|SetTool 4)))

(event Input|MouseEvents|RightMouseButton
  (params (Key :type Key%20Structure :default "None"))
  (bind _returnvalue (HUD|GetHUD))
  (bind _ashud_bear_grillz (Utilities|Casting|CastToHUD_BearGrillz _returnvalue))
  ;[1 1 1] Tools Menu
  (:Pressed
    (Default|SetToolsVisibility _ashud_bear_grillz true)
    (Input|SetInputModeUIOnly self (Variables|/Game/HF/Blueprints/Core/HUD_BearGrillz.HUD_BearGrillz_C|GetGameplayHUD _ashud_bear_grillz) "LockAlways" false))
  (:Released
    (Default|SetToolsVisibility _ashud_bear_grillz false)
    (Input|SetInputModeGameOnly self false)))

(fn ConstructionScript)

(fn GetCurrentTool
  (return (Utilities|Array|Get(acopy) (Variables|Default|GetTools) (Variables|Default|GetCurrentTool))))