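; HUD Blueprint that manages the game's screen widgets and the gameplay HUD, including its timer and tools display.
; GetWidgetOfClass creates each widget once and caches it by class, and OpenWidget stacks it, hides the gameplay HUD and sets UI-only input.
; Collapsing the top widget closes it through a visibility-changed binding, then reopens the one beneath or fires OnCloseAllWidgets and restores the gameplay HUD.
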(event Custom|SetToolsVisibility
  (params (Show :type Boolean))
  (bind _gameplayhud (Variables|Default|GetGameplayHUD))
  (if Show
    (Default|ShowTools _gameplayhud)
    (else
      (Default|HideTools _gameplayhud))))

(event Custom|OnLastWidgetOpenVisiblityChanged_Event
  (params (InVisibility :type ESlateVisibility%20Enum :default "Visible"))
  (bind _showingwidgets (Variables|Default|GetShowingWidgets))
  (bind _showingwidgets_2 (Variables|Default|GetShowingWidgets))
  (bind _showingwidgets_3 (Variables|Default|GetShowingWidgets))
  (switch Utilities|FlowControl|Switch|SwitchonESlateVisibility InVisibility
    (:Collapsed
      (if (Utilities|Array|IsNotEmpty (Variables|Default|GetShowingWidgets))
        (Widget|RemovefromParent (Utilities|Array|Get(acopy) _showingwidgets (Utilities|Array|LastIndex _showingwidgets)))
        (Utilities|Array|RemoveIndex _showingwidgets_3 (Utilities|Array|LastIndex _showingwidgets_3))
        (if (Utilities|Array|IsEmpty (Variables|Default|GetShowingWidgets))
          (Default|CallOnCloseAllWidgets)
          (bind _gameplayhud (Variables|Default|GetGameplayHUD)
            (:then
              (Widget|SetVisibility _gameplayhud "SelfHitTestInvisible"))
            (:else))
          (else
            (CallFunction|ReOpenWidget (Utilities|Array|Get(acopy) _showingwidgets_2 (Utilities|Array|LastIndex _showingwidgets_2)))))))))

(event Custom|ShowTimer
  (params (Timer :type Integer))
  (bind _gameplayhud (Variables|Default|GetGameplayHUD)
    (:then
      (Default|StartTimer _gameplayhud Timer))
    (:else)))

(event Custom|ShowGameplayScreen
  (bind _widget (CallFunction|GetWidgetOfClass "/Game/HF/Widgets/WBP_GameplayHUD.WBP_GameplayHUD_C"))
  (UserInterface|Viewport|AddtoViewport _widget 0)
  (bind _aswbp_gameplay_hud (Utilities|Casting|CastToWBP_GameplayHUD _widget))
  (Variables|Default|SetGameplayHUD _aswbp_gameplay_hud))

(fn ConstructionScript)

(fn GetWidgetOfClass
  (params (WidgetClass :type User%20Widget%20Class%20Reference))
  (bind _createdwidgets (Variables|Default|GetCreatedWidgets))
  (bind (_value _returnvalue) (Utilities|Map|Find _createdwidgets WidgetClass))
  (if _returnvalue
    (return _value)
    (else
      (bind _returnvalue_2 (UserInterface|CreateWidget WidgetClass (Game|GetPlayerController 0)))
      (Utilities|Map|Add (Variables|Default|GetCreatedWidgets) WidgetClass _returnvalue_2)
      (Widget|SetVisibility _returnvalue_2 "Collapsed")
      (return _returnvalue_2))))

(fn ReOpenWidget
  (params (WidgetToReopen :type User%20Widget%20Object%20Reference%20%28by%20ref%29))
  (if (Utilities|Array|ContainsItem (Variables|Default|GetShowingWidgets) WidgetToReopen)
    (UserInterface|Viewport|AddtoViewport WidgetToReopen 0)
    (Widget|SetVisibility WidgetToReopen "SelfHitTestInvisible")
    (EventDispatchers|BindEventtoOnVisibilityChanged WidgetToReopen (EventDispatchers|CreateEvent :!event Custom|OnLastWidgetOpenVisiblityChanged_Event))
    (Input|SetInputModeUIOnly (Game|Player|GetOwningPlayerController) WidgetToReopen "DoNotLock" false)))

(fn OpenWidget
  (params (WidgetClass :type User%20Widget%20Class%20Reference))
  (bind _showingwidgets (Variables|Default|GetShowingWidgets))
  (bind _widget (CallFunction|GetWidgetOfClass WidgetClass))
  (Variables|Default|SetUsingWidget _widget)
  (if (not (Utilities|Array|ContainsItem (Variables|Default|GetShowingWidgets) (Variables|Default|GetUsingWidget)))
    (Utilities|FlowControl|Sequence
      (:then_0
        (bind _gameplayhud (Variables|Default|GetGameplayHUD)
          (:then
            (Widget|SetVisibility _gameplayhud "Collapsed"))
          (:else)))
      (:then_1
        (if (Utilities|Array|IsNotEmpty (Variables|Default|GetShowingWidgets))
          (EventDispatchers|UnbindEventfromOnVisibilityChanged (Utilities|Array|Get(acopy) _showingwidgets (Utilities|Array|LastIndex _showingwidgets)) (EventDispatchers|CreateEvent :!event Custom|OnLastWidgetOpenVisiblityChanged_Event))))
      (:then_2
        (Utilities|Array|Add (Variables|Default|GetShowingWidgets) (Variables|Default|GetUsingWidget))
        (UserInterface|Viewport|AddtoViewport (Variables|Default|GetUsingWidget) 0)
        (Widget|SetVisibility (Variables|Default|GetUsingWidget) "SelfHitTestInvisible")
        (EventDispatchers|BindEventtoOnVisibilityChanged (Variables|Default|GetUsingWidget) (EventDispatchers|CreateEvent :!event Custom|OnLastWidgetOpenVisiblityChanged_Event))
        (Input|SetInputModeUIOnly (Game|Player|GetOwningPlayerController) (Variables|Default|GetUsingWidget) "DoNotLock" false)))))