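; Game mode for BearGrillz that runs the opening UI sequence when play begins.
; A tick after BeginPlay it gets the player's BearGrillz HUD and opens the main menu, then dialogue, then the tasks widget.
; Each step chains off the HUD's close-all-widgets event by swapping bindings.
; When the tasks widget closes, it switches to game-only input with permanent mouse capture on the next tick.
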(event EventBeginPlay
  (|CallParentFunction)
  (Utilities|FlowControl|DelayUntilNextTick)
  (CallFunction|StartGameLoop))

(event Custom|StartGameLoop
  (bind _ashud_bear_grillz (Utilities|Casting|CastToHUD_BearGrillz (HUD|GetHUD (Game|GetPlayerController 0))))
  (bind _output_get (Variables|Default|SetBearGrillzHUD _ashud_bear_grillz))
  (EventDispatchers|BindEventtoOnCloseAllWidgets _output_get (EventDispatchers|CreateEvent :!event Custom|OnCloseInitialMenu_Event))
  (Default|OpenWidget _output_get "/Game/HF/Widgets/WBP_MainMenu.WBP_MainMenu_C"))

(event Custom|OnCloseInitialTasksWidget_Event
  (EventDispatchers|UnbindEventfromOnCloseAllWidgets (Variables|Default|GetBearGrillzHUD) (delegate Custom|OnCloseInitialTasksWidget_Event))
  (Utilities|FlowControl|DelayUntilNextTick)
  (Input|SetInputModeGameOnly (Game|GetPlayerController 0) true)
  (Class|GameplayStatics|SetViewportMouseCaptureMode "CapturePermanently_IncludingInitialMouseDown"))

(event Custom|OnCloseInitialMenu_Event
  (EventDispatchers|UnbindEventfromOnCloseAllWidgets (Variables|Default|GetBearGrillzHUD) (delegate Custom|OnCloseInitialMenu_Event))
  (EventDispatchers|BindEventtoOnCloseAllWidgets (Variables|Default|GetBearGrillzHUD) (EventDispatchers|CreateEvent :!event Custom|OnCloseDialogue_Event))
  (Default|OpenWidget (Variables|Default|GetBearGrillzHUD) "/Game/HF/Widgets/WBP_Dialogue.WBP_Dialogue_C"))

(event Custom|OnCloseDialogue_Event
  (EventDispatchers|UnbindEventfromOnCloseAllWidgets (Variables|Default|GetBearGrillzHUD) (delegate Custom|OnCloseDialogue_Event))
  (EventDispatchers|BindEventtoOnCloseAllWidgets (Variables|Default|GetBearGrillzHUD) (EventDispatchers|CreateEvent :!event Custom|OnCloseInitialTasksWidget_Event))
  (Default|OpenWidget (Variables|Default|GetBearGrillzHUD) "/Game/HF/Widgets/WBP_Tasks.WBP_Tasks_C"))

(fn ConstructionScript)