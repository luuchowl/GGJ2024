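; Tool Blueprint that places a BP_Tooth actor at the point where it interacts.
; Interact runs the parent logic, then spawns the tooth at the hit location, scaled uniformly by Size.
; Roll and yaw are randomized within narrow ranges, while pitch flips the tooth 180 degrees unless the hit lies below a fixed world height, rather than following the surface normal.
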(event EventBeginPlay)

(event EventTick
  (params (DeltaSeconds :type Float%20%28single-precision%29)))

(fn Interact
  (params (HitResult :type Hit%20Result%20Structure))
  (bind (_bblockinghit _binitialoverlap _time _distance _location _impactpoint _normal) (Collision|BreakHitResult HitResult))
  (|CallParentFunction HitResult)
  (Game|SpawnActorfromClass "/Game/HF/Blueprints/BP_Tooth.BP_Tooth_C" (Math|Transform|MakeTransform _location (Math|Rotator|MakeRotator (Math|Random|RandomFloatinRange 0.0 1e+01) (Math|Float|SelectFloat 0.0 1.8e+02 (< (.Z (Math|Vector|BreakVector _location)) 4e+02)) (Math|Random|RandomFloatinRange 75.0 132.0)) (Math|Conversions|ToVector(Float) (Variables|Default|GetSize))) "Undefined" "MultiplyWithRoot" 0 0))