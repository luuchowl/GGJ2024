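; TOOL_Brackets is a tool Blueprint that places brackets where the player interacts and links consecutive ones.
; Interact spawns a BP_BracketLink at the hit location, appends it to Brackets and increments Count.
; From the second placement on, it spawns another, untracked BP_BracketLink at the midpoint of the last two, rotated along their line and stretched in X by their distance.
; A leftover "Hello" debug print fires on each link.
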(event EventBeginPlay
  (|CallParentFunction) ; This node is disabled and will not be called.\nDrag off pins to build functionality.
)

(event EventTick
  (params (DeltaSeconds :type Float%20%28single-precision%29))
  (|CallParentFunction DeltaSeconds) ; This node is disabled and will not be called.\nDrag off pins to build functionality.
)

(fn Interact
  (params (HitResult :type Hit%20Result%20Structure))
  (bind _brackets (Variables|Default|GetBrackets))
  (bind _count (Variables|Default|GetCount))
  (bind _count_2 (Variables|Default|GetCount))
  (bind _brackets_2 (Variables|Default|GetBrackets))
  (bind _returnvalue (- _count_2 1))
  (bind _returnvalue_2 (- _count 2))
  (bind _output (Utilities|Array|Get(acopy) _brackets _returnvalue))
  (bind _output_2 (Utilities|Array|Get(acopy) _brackets_2 _returnvalue_2))
  (bind _returnvalue_3 (Transformation|GetActorLocation _output))
  (bind _returnvalue_4 (Transformation|GetActorLocation _output_2))
  (|CallParentFunction HitResult)
  (bind _returnvalue_5 (Game|SpawnActorfromClass "/Game/HF/Blueprints/BP_BracketLink.BP_BracketLink_C" (Math|Transform|MakeTransform (.Location (Collision|BreakHitResult HitResult))) "Undefined" "MultiplyWithRoot" 0 0))
  (Utilities|Array|Add (Variables|Default|GetBrackets) _returnvalue_5)
  (bind _result (Math|Integer|IncrementInt (Variables|Default|GetCount))
    (:%20%20
      (if (>= _result 2)
        (Development|PrintString "Hello")
        (Game|SpawnActorfromClass "/Game/HF/Blueprints/BP_BracketLink.BP_BracketLink_C" (Math|Transform|MakeTransform (Math|Vector|Lerp(Vector) _returnvalue_4 _returnvalue_3 0.5) (Math|Rotator|FindLookatRotation _returnvalue_4 _returnvalue_3) (Math|Vector|MakeVector (* (Math|Vector|Distance(Vector) _returnvalue_4 _returnvalue_3) 0.2) 0.2 0.2)) "Undefined" "MultiplyWithRoot" 0 0)))))